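; Player camera pawn that drives its SMSphere component steadily forward while a player controls it.
; Tick checks IsPlayerControlled and passes delta time to PlayerControls.
; PlayerControls moves the sphere along its own forward vector at a fixed, frame-rate-independent speed, reading no input and using no collision sweep.
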(event EventBeginPlay)

(event Collision|EventActorBeginOverlap
  (params (OtherActor :type Actor%20Object%20Reference)))

(event EventTick
  (params (DeltaSeconds :type Float%20%28single-precision%29))
  (if (Pawn|IsPlayerControlled)
    (CallFunction|PlayerControls DeltaSeconds)))

(fn ConstructionScript)

(fn PlayerControls
  (params (deltaTime :type Float%20%28single-precision%29))
  (bind _sm_sphere (Variables|Default|GetSM_Sphere))
  (LocalVariables|SetΔT deltaTime)
  (Utilities|FlowControl|Sequence
    (:then_0
      (Transformation|SetWorldLocation _sm_sphere (+ (Transformation|GetWorldLocation _sm_sphere) (* (* (Math|Vector|GetForwardVector _sm_sphere) 5e+02) (LocalVariables|GetΔT))) false false))))